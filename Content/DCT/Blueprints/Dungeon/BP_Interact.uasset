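; Base dungeon interactable that toggles between Pre and Post Interact states, with optional single-use and reversed power.
; Click boxes gate interaction and rim-light hover highlighting, while step boxes toggle state as dungeon pawns finish steps on or off them.
; PowerActors relays state to linked actors, and an empty UpdateStateInstantly hook receives state updates.
; It also snaps to the grid index, attaches to slots, saves state and lerps cameras to a peek arrow.
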(event Custom|Peak
  (params (PeakTarget :type Actor%20Object%20Reference) (Playtime :type Float%20%28double-precision%29))
  (bind _returnvalue (Actor|GetComponentbyClass PeakTarget "/Script/Engine.CameraComponent"))
  (bind ___ (Utilities|MakeLocalVariable (Transformation|GetWorldTransform _returnvalue)))
  (bind _alpha (Utilities|SmoothLerp Playtime "/Game/DCT/Data/Curve_Smooth_Float.Curve_Smooth_Float" 1.0 false false)
    (:Update
      (Transformation|SetWorldTransform _returnvalue (Math|Transform|Lerp(Transform) ___ (Transformation|GetWorldTransform (Variables|Default|GetPeakArrow)) _alpha) false false))))

(event Custom|PowerActors
  (params (DesiredState :type EInteractState%20Enum :default "NewEnumerator0"))
  (for _array_element (Variables|Default|GetPoweredActors)
    (Class|BPIInteract|Power(Message) _array_element self DesiredState)))

(event Custom|UpdateStateInstantly
  (params (DesiredState :type EInteractState%20Enum :default "NewEnumerator0")))

(event Custom|Highlight
  (params (bEnable :type Boolean))
  (Variables|Default|SetbHighlighted bEnable)
  (for _array_element (Variables|Default|GetDynamicMaterials)
    (Rendering|Material|SetScalarParameterValue _array_element "RimlightStrength" (Math|Conversions|ToFloat(Boolean) (Variables|Default|GetbHighlighted)) :!class /Script/Engine.MaterialInstanceDynamic)))

(event Custom|CallOnPlayerStepEnd
  (params (DungeonPawn :type BP%20Dungeon%20Pawn%20Object%20Reference))
  (bind _desiredstate (Variables|Default|GetDesiredState))
  (bind _boverlaps (CallFunction|DoesActorOverlapCollisionBoxwithTag DungeonPawn "Step"))
  (if _boverlaps
    (switch Utilities|FlowControl|Switch|SwitchonEInteractState _desiredstate
      (:NewEnumerator0
        (CallFunction|Interact DungeonPawn :!label _label)))
    (else
      (switch Utilities|FlowControl|Switch|SwitchonEInteractState _desiredstate
        (:NewEnumerator2
          (Utilities|FlowControl|Sequence
            (:then_0
              (goto _label))
            (:then_1
              (EventDispatchers|UnbindEventfromOnStepEnd DungeonPawn (delegate Custom|CallOnPlayerStepEnd)))))))))

(event EventInteract
  (params (TriggeringActor :type Actor%20Object%20Reference))
  (bind _output_get (Variables|Default|SetDesiredState (CallFunction|GetOppositeInteractState (Variables|Default|GetDesiredState))))
  (CallFunction|Power 0 _output_get))

(event MouseInput|EventActorBeginCursorOver
  (if (Variables|Default|GetbEnableHighlight)
    (Variables|Default|SetbCursorOver true)
    (Utilities|WhileLoopDelayed (Variables|Default|GetbCursorOver) 0.1
      (:Loop%20Body
        (bind _ballowed (CallFunction|CheckifAllowedInteract (Game|Player|GetPlayerPawn 0)))
        (if (!= _ballowed (Variables|Default|GetbHighlighted))
          (CallFunction|Highlight _ballowed))))))

(event MouseInput|EventActorEndCursorOver
  (if (Variables|Default|GetbEnableHighlight)
    (Variables|Default|SetbCursorOver false)
    (CallFunction|Highlight false)))

(event EventSaveActor
  (params (DungeonInstance :type BP%20GI%20Dungeon%20Object%20Reference))
  (bind _self self)
  (Utilities|Array|Add (Variables|/Game/DCT/Blueprints/Core/BP_GI_Dungeon.BP_GI_Dungeon_C|GetSavedInteractables DungeonInstance) (Utilities|Struct|MakeFInteractableSave (Utilities|GetDisplayName _self) (Transformation|GetActorTransform) (Variables|Default|GetDesiredState) (Utilities|GetClass _self))))

(event Collision|EventActorBeginOverlap
  (params (OtherActor :type Actor%20Object%20Reference))
  (if (> (Utilities|Array|Length (Variables|Default|GetInteractionStepAreas)) 0)
    (bind _asbp_dungeon_pawn (Utilities|Casting|CastToBP_DungeonPawn OtherActor))
    (EventDispatchers|BindEventtoOnStepEnd _asbp_dungeon_pawn (delegate Custom|CallOnPlayerStepEnd))))

(event EventBeginPlay
  (Variables|Default|SetOriginalState (Variables|Default|GetDesiredState))
  (CallFunction|AttachtoSelectedSlotifValid)
  (Utilities|FlowControl|Sequence
    (:then_0
      (if (Variables|Default|GetbEnableHighlight)
        (for _array_element (Actor|GetComponentsByClass "/Script/Engine.StaticMeshComponent")
          (for (_array_element_2 _array_index) (Rendering|Material|GetMaterials _array_element)
            (bind _returnvalue (Rendering|Material|CreateDynamicMaterialInstance _array_element _array_index _array_element_2 "None" :!class /Script/Engine.PrimitiveComponent))
            (Utilities|Array|Add (Variables|Default|GetDynamicMaterials) _returnvalue)))))
    (:then_1
      (Utilities|FlowControl|Delay 0.0)
      (bind _gridindex (Default|FindNearbyValidTile (.DungeonManager (CallFunction|GetDungeonManager)) (Transformation|GetActorLocation)))
      (Variables|Default|SetGridIndex _gridindex))))

(event EventUpdateDesiredState
  (params (NewState :type EInteractState%20Enum :default "NewEnumerator0"))
  (bind _output_get (Variables|Default|SetDesiredState NewState))
  (if (Utilities|Enum|NotEqual(Enum) (Variables|Default|GetInteractState) _output_get)
    (bind _output_get_2 (Variables|Default|SetInteractState _output_get))
    (CallFunction|UpdateStateInstantly _output_get_2)))

(event EventPower
  (params (TriggeringActor :type Actor%20Object%20Reference) (DesiredState :type EInteractState%20Enum :default "NewEnumerator0"))
  (if (Variables|Default|GetbReversedPower)
    (Variables|Default|SetDesiredState (CallFunction|GetOppositeInteractState DesiredState))
    (else
      (Variables|Default|SetDesiredState DesiredState))))

(fn ConstructionScript
  (Rendering|SetVisibility (Variables|Default|GetPeakArrow) (Variables|Default|GetbShowPeakArrow) false)
  (for _array_element (Variables|Default|GetInteractionClickAreas)
    (AddComponent|AddBoxComponent false _array_element))
  (for _array_element_2 (Variables|Default|GetInteractionStepAreas)
    (AddComponent|AddBoxComponent false _array_element_2))
  (CallFunction|UpdateDesiredState (Variables|Default|GetDesiredState)))

(fn GetOppositeInteractState
  (params (Index :type EInteractState%20Enum :default "NewEnumerator0"))
  (return (Utilities|Select :Index Index :NewEnumerator0 "NewEnumerator2" :NewEnumerator2 "NewEnumerator0")))

(fn DoesActorOverlapCollisionBoxwithTag
  (params (Actor :type Actor%20Object%20Reference) (CollisionBoxTag :type Name :default "Click"))
  (for _array_element (Class|Actor|GetOverlappingComponents Actor)
    (bind _asbox_collision (Utilities|Casting|CastToBoxComponent _array_element))
    (if (Utilities|Array|ContainsItem (Actor|GetComponentsbyTag "/Script/Engine.BoxComponent" CollisionBoxTag) _asbox_collision)
      (return true)))
  (return false))

(fn AttachtoSelectedSlotifValid
  (bind _attachslot (Class|BPIInteract|GetAttachSlot(Message) (Variables|Default|GetActorToAttach)))
  (Utilities|IsValid _attachslot
    (:Is%20Valid
      (Transformation|AttachComponentToComponent _attachslot "None" "KeepWorld" "KeepWorld" "KeepWorld" true)
      (return true))
    (:Is%20Not%20Valid
      (return true))))

(fn CheckifExhausted
  (return (and (Variables|Default|GetbSingleUse) (!= (Variables|Default|GetOriginalState) (Variables|Default|GetInteractState)))))

(fn AttemptInteract
  (params (TriggeringActor :type Actor%20Object%20Reference))
  (if (not (CallFunction|CheckifExhausted))
    (bind _ballowed (CallFunction|CheckifAllowedInteract TriggeringActor))
    (if _ballowed
      (bind _output_get (Variables|Default|SetTriggeringActor TriggeringActor))
      (CallFunction|Interact _output_get)
      (return true)
      (else
        (return false)))
    (else
      (return false))))

(fn CheckifAllowedInteract
  (params (TriggeringActor :type Actor%20Object%20Reference))
  (if (or (Variables|Default|GetbAllowInteractDuringTransition) (== (Variables|Default|GetInteractState) (Variables|Default|GetDesiredState)))
    (Utilities|IsValid TriggeringActor
      (:Is%20Valid
        (bind _aspawn (Utilities|Casting|CastToPawn TriggeringActor)
          (:then
            (bind _boverlaps (CallFunction|DoesActorOverlapCollisionBoxwithTag _aspawn "Click"))
            (return _boverlaps))
          (:CastFailed
            (return true))))
      (:Is%20Not%20Valid
        (return true)))
    (else
      (return false))))

(fn GetAttachSlot
  (return 0))