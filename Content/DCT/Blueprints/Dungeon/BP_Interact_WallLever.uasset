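; BP_Interact_WallLever is a dungeon wall lever that switches between pre- and post-interact states to power other actors.
; Its Power event plays or reverses the TL_Press timeline, which rotates the lever mesh around its roll axis.
; When the timeline finishes, it plays a switch sound, stores the new InteractState and calls PowerActors with it.
; UpdateStateInstantly sets the timeline time directly to change state without the normal press.
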(event EventPower
  (params (TriggeringActor :type Actor%20Object%20Reference) (DesiredState :type EInteractState%20Enum :default "NewEnumerator0"))
  (bind _output_get (Variables|Default|SetDesiredState DesiredState))
  (switch Utilities|FlowControl|Switch|SwitchonEInteractState _output_get
    (:NewEnumerator0
      (bind _rotate (Timeline|TL_Press Reverse)
        (:Update
          (Transformation|SetRelativeRotation (Variables|Default|GetLever) (Math|Rotator|MakeRotator _rotate 0.0 0.0) false false))
        (:Finished
          (Audio|PlaySoundatLocation "/Game/DCT/Sound/A_Switch.A_Switch" (Transformation|GetActorLocation) "0, 0, 0" 1.0 1.0 0.0 "/Game/DCT/Sound/ATT_Dungeon.ATT_Dungeon" 0 0 0)
          (bind _output_get_2 (Variables|Default|SetInteractState (Variables|Default|GetDesiredState)))
          (CallFunction|PowerActors _output_get_2))))
    (:NewEnumerator2
      (Timeline|TL_Press Play))))

(event EventUpdateStateInstantly
  (params (DesiredState :type EInteractState%20Enum :default "NewEnumerator0"))
  (bind _rotate (Timeline|TL_Press SetNewTime)
    (:Update
      (Transformation|SetRelativeRotation (Variables|Default|GetLever) (Math|Rotator|MakeRotator _rotate 0.0 0.0) false false))
    (:Finished
      (Audio|PlaySoundatLocation "/Game/DCT/Sound/A_Switch.A_Switch" (Transformation|GetActorLocation) "0, 0, 0" 1.0 1.0 0.0 "/Game/DCT/Sound/ATT_Dungeon.ATT_Dungeon" 0 0 0)
      (bind _output_get (Variables|Default|SetInteractState (Variables|Default|GetDesiredState)))
      (CallFunction|PowerActors _output_get))))

(fn ConstructionScript)