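; Dungeon NPC that varies its look at spawn, snaps to a nearby valid tile and barks at the player.
; The bark trigger shows a random-line widget and turns the mesh toward BP_DungeonPawn each tick until overlap ends.
; Grid pathfinding toward AuctionUnit goes through BP_DungeonManager, but movement is unfinished.
; UpdateMove's call here is unwired, and the step, rotate and grid-registration functions are stubs or incomplete.
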(event OnComponentBeginOverlap(BarkTrigger)
  (params (OverlappedComponent :type Primitive%20Component%20Object%20Reference) (OtherActor :type Actor%20Object%20Reference) (OtherComp :type Primitive%20Component%20Object%20Reference) (OtherBodyIndex :type Integer) (bFromSweep :type Boolean) (SweepResult :type Hit%20Result%20Structure%20%28by%20ref%29))
  (bind _barksentences (Variables|Default|GetBarkSentences))
  (Utilities|Casting|CastToBP_DungeonPawn OtherActor)
  (bind _returnvalue (UserInterface|CreateWidget "/Game/Dynamic/Blueprints/BarkUI/WBP_BarkUI.WBP_BarkUI_C"))
  (Default|InitialiseBark _returnvalue (Variables|Default|GetName) (Utilities|Array|Get(acopy) _barksentences (Math|Random|RandomInteger (Utilities|Array|Length _barksentences))))
  (UserInterface|Viewport|AddtoViewport _returnvalue 3)
  (Variables|Default|SetBarkWidget _returnvalue)
  (Variables|Default|SetTalkingToPlayer true))

(event OnComponentEndOverlap(BarkTrigger)
  (params (OverlappedComponent :type Primitive%20Component%20Object%20Reference) (OtherActor :type Actor%20Object%20Reference) (OtherComp :type Primitive%20Component%20Object%20Reference) (OtherBodyIndex :type Integer))
  (bind _barkwidget (Variables|Default|GetBarkWidget))
  (Variables|Default|SetTalkingToPlayer false)
  (Transformation|SetWorldRotation (Variables|Default|GetSkeletalMesh) (Variables|Default|GetStartRotation) false false)
  (UserInterface|Animation|PlayAnimation _barkwidget (Variables|/Game/Dynamic/Blueprints/BarkUI/WBP_BarkUI.WBP_BarkUI_C|GetFadeOut _barkwidget) 0.0 1 "Forward" 1.0 false)
  (Utilities|FlowControl|Delay 0.25)
  (Widget|RemovefromParent _barkwidget))

(event Custom|UpdateMove
  (params (Use%20Shared%20Path :type Boolean))
  (if (not (or (Variables|Default|GetbDead) (Variables|Default|GetbIdle)))
    (bind (_pathfound _path _path_indexes) (CallFunction|FindPathtoAuction))
    (if _pathfound
      (Variables|Default|SetCurrent%20Path%20Indexes _path_indexes)
      (bind _output_get (Variables|Default|SetCurrent%20Path _path))
      (Utilities|Array|RemoveIndex _output_get (Utilities|Array|LastIndex _output_get))
      (CallFunction|MovePath (Variables|Default|GetCurrent%20Path)))))

(event Custom|MovePath
  (params (Path :type Array%20of%20Vectors))
  (Variables|Default|SetCurrent%20Path Path)
  (if (> (Utilities|Array|Length (Variables|Default|GetCurrent%20Path)) 0)
    (if (Utilities|Operators|NotEqual(!=) (CallFunction|GetNextPathLocation) (Transformation|GetActorLocation) 1.0)
      (if (CallFunction|IsUnitonLocation "0, 0, 0")
        _)
      (else
        (Utilities|Array|RemoveIndex (Variables|Default|GetCurrent%20Path) (Utilities|Array|LastIndex (Variables|Default|GetCurrent%20Path)))
        (CallFunction|MovePath (Variables|Default|GetCurrent%20Path))))))

(event Custom|RotateTowardsLocation
  (params (TargetLocation :type Vector))
  (bind _returnvalue (Transformation|GetActorLocation))
  (bind (_x _y) (Math|Vector|BreakVector TargetLocation))
  (Utilities|MakeLocalVariable (Transformation|GetActorRotation))
  (Utilities|MakeLocalVariable (Math|Rotator|FindLookatRotation (Math|Vector|MakeVector (.x _returnvalue) (.y _returnvalue) 0.0) (Math|Vector|MakeVector _x _y 0.0))))

(event Custom|StepToLocation
  (params (TargetLocation :type Vector))
  (Utilities|MakeLocalVariable TargetLocation)
  (Utilities|MakeLocalVariable (Transformation|GetActorLocation)))

(event EventBeginPlay
  (bind _skeletalmesh (Variables|Default|GetSkeletalMesh))
  (bind _skeletalmesh_2 (Variables|Default|GetSkeletalMesh))
  ;[0 0 0] Setup
  (if (Variables|Default|GetUseRandomMat)
    (Rendering|Material|SetMaterial _skeletalmesh 0 (.OutItem (Utilities|Array|Random (Variables|Default|GetMatArray)))))
  (Components|SkeletalMesh|SetMorphTarget _skeletalmesh "Scrawny" (Math|Random|RandomFloatinRange -1.0 1.0) true)
  (Utilities|FlowControl|Delay 0.2)
  (bind _returnvalue (Actor|GetActorOfClass "/Game/DCT/Blueprints/Core/BP_DungeonManager.BP_DungeonManager_C"))
  (Variables|Default|SetDungeonManager _returnvalue)
  (bind _tilelocation (Default|FindNearbyValidTile (Variables|Default|GetDungeonManager) (Transformation|GetActorLocation)))
  (Transformation|SetActorLocation _tilelocation false false)
  (Variables|Default|SetStartRotation (Transformation|GetWorldRotation (Variables|Default|GetSkeletalMesh)))
  (Audio|Components|Audio|Stop _skeletalmesh_2)
  (Utilities|FlowControl|Delay (Math|Random|RandomFloatinRange 0.0 1.0))
  (Audio|Components|Audio|Play _skeletalmesh_2 true))

(event EventTick
  (params (DeltaSeconds :type Float%20%28single-precision%29))
  (if (Variables|Default|GetTalkingToPlayer)
    (CallFunction|LookatPlayer)))

(fn ConstructionScript)

(fn FindPathtoAuction
  (bind (_pathsmap _auctionfound _auctiongridindex) (CallFunction|SearchforAuction))
  (if _auctionfound
    (bind _pathindexes (Default|FindPathtoIndex (Variables|Default|GetDungeonManager) _pathsmap _auctiongridindex))
    (bind _output_get (LocalVariables|SetLocal%20Path%20Indexes _pathindexes))
    (bind _locations (Default|ConvertGridIndexestoLocations (Variables|Default|GetDungeonManager) _output_get "0, 0, 0"))
    (bind _inverted_path (CallFunction|InvertPath _locations))
    (return true _inverted_path (LocalVariables|GetLocal%20Path%20Indexes))))

(fn SearchforAuction
  (bind _dungeonmanager (Variables|Default|GetDungeonManager))
  (bind _auctionunit (Variables|Default|GetAuctionUnit))
  (bind _returnvalue (Transformation|GetActorLocation _auctionunit))
  (bind _gridindex (Default|ConvertLocationtoIndex _dungeonmanager _returnvalue))
  (bind (_pathsmap _btargetfound) (Default|RunPathfinding (Variables|Default|GetDungeonManager) (Default|ConvertLocationtoIndex (Variables|Default|GetDungeonManager) (Transformation|GetActorLocation)) (Variables|Default|GetMoveSearchRange) _gridindex true))
  (return _pathsmap _btargetfound _gridindex))

(fn InvertPath
  (params (Path%20In :type Array%20of%20Vectors))
  (bind _arrayelement (Utilities|Array|ReverseforEachLoop Path%20In)
    (:LoopBody
      (Utilities|Array|Add (LocalVariables|GetLocal%20Path) _arrayelement))
    (:Completed
      (return (LocalVariables|GetLocal%20Path)))))

(fn GetNextPathLocation
  (bind _current_path (Variables|Default|GetCurrent%20Path))
  (return (Utilities|Array|Get(acopy) _current_path (Utilities|Array|LastIndex _current_path))))

(fn IsUnitonLocation
  (params (Location :type Vector))
  (return (!= (Default|ConvertLocationtoIndex (Variables|Default|GetDungeonManager) "0, 0, 0") (Default|ConvertLocationtoIndex (Variables|Default|GetDungeonManager) Location))))

(fn MoveNPConGrid
  (params (TargetLocation :type Vector))
  (CallFunction|RemoveNPCfromGrid)
  (Default|FindNearbyValidTile (Variables|Default|GetDungeonManager) TargetLocation))

(fn RemoveNPCfromGrid
  (Default|RemoveObjectfromGrid (Variables|Default|GetDungeonManager) self (Variables|Default|GetGrid%20Index))
  (return))

(fn AddNPCtoGrid
  (params (GridIndex :type Integer))
  (Variables|Default|SetGrid%20Index GridIndex))

(fn AddObjecttoGrid)

(fn LookatPlayer
  (bind _outactors (Actor|GetAllActorsOfClass "/Game/DCT/Blueprints/Core/BP_DungeonPawn.BP_DungeonPawn_C"))
  (Transformation|SetWorldRotation (Variables|Default|GetSkeletalMesh) (Math|Rotator|MakeRotator (.roll (Math|Rotator|FindLookatRotation (Transformation|GetActorLocation) (Transformation|GetActorLocation (Utilities|Array|Get(acopy) _outactors)))) (.pitch (Math|Rotator|FindLookatRotation (Transformation|GetActorLocation) (Transformation|GetActorLocation (Utilities|Array|Get(acopy) _outactors)))) (+ (.yaw (Math|Rotator|FindLookatRotation (Transformation|GetActorLocation) (Transformation|GetActorLocation (Utilities|Array|Get(acopy) _outactors)))) -9e+01)) false false))