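; BP_UnitManager controls which BP_Interact_Unit actors in the level have an active auction, starting with one random unit at BeginPlay.
; ActivateUnits shuffles either all units or the not-yet-used pool, removes its picks from that pool, and sets every unit's auction active or inactive.
; ReActivateAuctions draws the next non-repeating unit and shows the WinScreen widget when the pool is exhausted.
; DeactivateAllUnits is an empty, unused stub.
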(event Custom|ReActivateAuctions
  (bind _finished (CallFunction|ActivateUnits 1 false))
  (if _finished
    (bind _returnvalue (UserInterface|CreateWidget "/Game/Dynamic/Blueprints/ResultsUIStuff/WinScreen.WinScreen_C"))
    (UserInterface|Viewport|AddtoViewport _returnvalue 2)))

(event EventBeginPlay
  (bind _outactors (Actor|GetAllActorsOfClass "/Game/Dynamic/Blueprints/BP_Interact_Unit.BP_Interact_Unit_C"))
  (bind _output_get (Variables|Default|SetUnits _outactors))
  (Variables|Default|SetPotentialUnits _output_get)
  (CallFunction|ActivateUnits 1 false))

(fn ConstructionScript)

(fn ActivateUnits
  (params (Number%20To%20Activate :type Integer) (Repeatable :type Boolean))
  (bind _unitstoactivate (LocalVariables|GetUnitsToActivate))
  (bind _potentialunits (Variables|Default|GetPotentialUnits))
  (if Repeatable
    (bind _output_get (LocalVariables|SetTempUnits (Variables|Default|GetUnits)))
    (Utilities|Array|Shuffle _output_get)
    (else
      (bind _output_get_2 (LocalVariables|SetTempUnits (Variables|Default|GetPotentialUnits)))
      (Utilities|Array|Shuffle _output_get_2)))
  (bind _index (Utilities|FlowControl|ForLoopwithBreak 0 (- Number%20To%20Activate 1) :!label _label)
    (:LoopBody
      (if (> _index (- (Utilities|Array|Length (LocalVariables|GetTempUnits)) 1))
        (LocalVariables|Setexhausted true)
        (goto _label Break)
        (else
          (Utilities|Array|Add (LocalVariables|GetUnitsToActivate) (Utilities|Array|Get(acopy) (LocalVariables|GetTempUnits) _index))
          (if (Utilities|Array|ContainsItem _potentialunits (Utilities|Array|Get(acopy) (LocalVariables|GetTempUnits) _index))
            (Utilities|Array|RemoveItem _potentialunits (Utilities|Array|Get(acopy) (LocalVariables|GetTempUnits) _index))))))
    (:Completed
      (for _array_element (Variables|Default|GetUnits)
        (if (Utilities|Array|ContainsItem _unitstoactivate _array_element)
          (Default|SetAuctionActive _array_element)
          (else
            (Default|SetAuctionInactive _array_element))))
      (Variables|Default|SetActiveUnits _unitstoactivate)
      (return (LocalVariables|Getexhausted)))))

(fn DeactivateAllUnits)