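; AuctionTreasure is a short-lived treasure actor that plays a flight animation for the auction UI, then destroys itself.
; It records the mesh's start position on BeginPlay.
; SpawnAnimation runs a brief SmoothLerp shaped by TreasureScaleCurve, using its alpha for uniform scale and horizontal movement up to halfway toward AuctionCameraLocation.
; FlightCurve, sampled with that same alpha, adds a height offset to the starting Z.
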(event Custom|SpawnAnimation
  (bind _staticmesh (Variables|Default|GetStaticMesh))
  (bind _alpha (Utilities|SmoothLerp 0.75 "/Game/Dynamic/Blueprints/AuctionUIStuff/TreasureScaleCurve.TreasureScaleCurve" 1.0 false false)
    (:Update
      (Transformation|SetWorldScale3D _staticmesh (Math|Conversions|ToVector(Float) _alpha))
      (Transformation|SetWorldLocation _staticmesh (Math|Vector|MakeVector (.x (Math|Vector|Lerp(Vector) (Variables|Default|GetStartPosition) (Variables|Default|GetAuctionCameraLocation) (/ _alpha 2.0))) (.y (Math|Vector|Lerp(Vector) (Variables|Default|GetStartPosition) (Variables|Default|GetAuctionCameraLocation) (/ _alpha 2.0))) (+ (* (Math|Curves|GetFloatValue (Variables|Default|GetFlightCurve) _alpha) 5e+01) (.z (Variables|Default|GetStartPosition)))) false false))
    (:Finished
      (Actor|DestroyActor))))

(event EventBeginPlay
  (Variables|Default|SetStartPosition (Transformation|GetWorldLocation (Variables|Default|GetStaticMesh))))

(fn ConstructionScript)