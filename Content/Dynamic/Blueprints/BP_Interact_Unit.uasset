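; Interactable dungeon storage unit door that sends the player into an auction when powered while active.
; Power shows a transition widget, switches to the auction camera and UI, and runs the door timeline alongside sound, collision and dungeon tile updates.
; SetAuctionActive/Inactive toggle interactability and door material.
; ReturnFromAuction restores the player view, increments the completed count and has BP_UnitManager reactivate auctions.
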(event Custom|SetAuctionActive
  (Rendering|Material|SetMaterial (Variables|Default|GetStorageDoor) 1 "/Game/Static/Textures/StorageUnits/storage_cluttered/clutter_unit.clutter_unit")
  (Variables|Default|SetInteractable true))

(event Custom|SetAuctionInactive
  (Rendering|Material|SetMaterial (Variables|Default|GetStorageDoor) 1 "/Game/Static/Models/ModularDungeon/M_storage_door.M_storage_door")
  (Variables|Default|SetInteractable false))

(event EventUpdateStateInstantly
  (params (DesiredState :type EInteractState%20Enum :default "NewEnumerator0"))
  (Variables|Default|SetDesiredState DesiredState)
  (Utilities|FlowControl|Sequence
    (:then_0
      (bind _open (Timeline|TL_Open SetNewTime)
        (:Finished
          (Utilities|FlowControl|Sequence
            (:then_0
              (Collision|SetCollisionEnabled (Variables|Default|GetWallBlockingBox) (Utilities|Select :Index (Variables|Default|GetDesiredState) :NewEnumerator0 "QueryOnly" :NewEnumerator2 "NoCollision") :!label _label))
            (:then_1
              (Audio|PlaySoundatLocation "/Game/DCT/Sound/A_DoorClose.A_DoorClose" (Transformation|GetActorLocation) "0, 0, 0" 1.0 1.0 0.0 "/Game/DCT/Sound/ATT_Dungeon.ATT_Dungeon" 0 0 0)
              (Default|UpdateTilesinRange (.DungeonManager (CallFunction|GetDungeonManager)) 2 0 (Transformation|GetActorLocation) false)
              (Variables|Default|SetInteractState (Variables|Default|GetDesiredState))
              (CallFunction|ForceMonstersLookforPlayer))))))
    (:then_1
      (goto _label))))

(event EventUpdateDesiredState
  (params (NewState :type EInteractState%20Enum :default "NewEnumerator0"))
  (|CallParentFunction NewState))

(event EventBeginPlay
  (|CallParentFunction)
  (Collision|SetCollisionEnabled (Variables|Default|GetWallBlockingBox) (Utilities|Select :Index (Variables|Default|GetDesiredState) :NewEnumerator0 "QueryOnly" :NewEnumerator2 "NoCollision")))

(event EventPower
  (params (TriggeringActor :type Actor%20Object%20Reference) (DesiredState :type EInteractState%20Enum :default "NewEnumerator0"))
  (if (Variables|Default|GetInteractable)
    (|CallParentFunction 0 DesiredState)
    (Collision|SetCollisionEnabled (Variables|Default|GetWallBlockingBox) "QueryAndPhysics")
    (Default|UpdateTilesinRange (.DungeonManager (CallFunction|GetDungeonManager)) 2 0 (Transformation|GetActorLocation) false)
    (Utilities|FlowControl|Sequence
      (:then_0
        (bind _returnvalue (UserInterface|CreateWidget "/Game/Dynamic/Blueprints/AuctionTestWidget.AuctionTestWidget_C"))
        (UserInterface|Viewport|AddtoViewport _returnvalue 1)
        (Utilities|FlowControl|Delay 0.5)
        (CallFunction|GotoAuction)
        (Utilities|FlowControl|Delay 0.5)
        (Widget|RemovefromParent _returnvalue))
      (:then_1
        (if (Audio|Components|Audio|IsPlaying (Variables|Default|GetTL_Open))
          _
          (else
            (Audio|PlaySoundatLocation "/Game/DCT/Sound/A_OpenDoor.A_OpenDoor" (Transformation|GetActorLocation) "0, 0, 0" 1.0 1.0 0.0 "/Game/DCT/Sound/ATT_Dungeon.ATT_Dungeon" 0 0 0)))
        (switch Utilities|FlowControl|Switch|SwitchonEInteractState (Variables|Default|GetDesiredState)
          (:NewEnumerator0
            (bind _open (Timeline|TL_Open Reverse)
              (:Finished
                (Utilities|FlowControl|Sequence
                  (:then_0
                    (Collision|SetCollisionEnabled (Variables|Default|GetWallBlockingBox) (Utilities|Select :Index (Variables|Default|GetDesiredState) :NewEnumerator0 "QueryOnly" :NewEnumerator2 "NoCollision")))
                  (:then_1
                    (Audio|PlaySoundatLocation "/Game/DCT/Sound/A_DoorClose.A_DoorClose" (Transformation|GetActorLocation) "0, 0, 0" 1.0 1.0 0.0 "/Game/DCT/Sound/ATT_Dungeon.ATT_Dungeon" 0 0 0)
                    (Default|UpdateTilesinRange (.DungeonManager (CallFunction|GetDungeonManager)) 2 0 (Transformation|GetActorLocation) false)
                    (Variables|Default|SetInteractState (Variables|Default|GetDesiredState))
                    (CallFunction|ForceMonstersLookforPlayer))))))
          (:NewEnumerator2
            (Timeline|TL_Open Play)))))))

(fn ConstructionScript
  (|CallParentFunction)
  (Collision|SetCollisionEnabled (Variables|Default|GetWallBlockingBox) (Utilities|Select :Index (Variables|Default|GetDesiredState) :NewEnumerator0 "QueryOnly" :NewEnumerator2 "NoCollision")))

(fn MoveDoor
  (params (PercentOpen :type Float%20%28double-precision%29))
  (Transformation|SetRelativeRotation (Variables|Default|GetPivot) (Math|Rotator|MakeRotator 0.0 0.0 (* PercentOpen 9e+01)) false false))

(fn GetAttachSlot
  (return (Variables|Default|GetAttachSlot)))

(fn GotoAuction
  (bind _returnvalue (Game|GetPlayerController 0))
  (bind _auction_camera (Variables|Default|GetAuction%20Camera))
  (Rendering|Material|SetMaterial (Variables|/Script/Engine.StaticMeshActor|GetStaticMeshComponent (Variables|Default|GetAuctionUnitMesh)) 1 "/Game/Static/Textures/StorageUnits/storage_cluttered/clutter_unit.clutter_unit")
  (if (Utilities|IsValid _auction_camera)
    (Game|Player|SetViewTargetwithBlend _returnvalue _auction_camera 0.0 "VTBlend_Linear" 0.0 false)
    (Input|SetInputModeUIOnly _returnvalue 0 "DoNotLock" false)
    (bind _returnvalue_2 (UserInterface|CreateWidget "/Game/Dynamic/Blueprints/AuctionUIStuff/AuctionUI.AuctionUI_C"))
    (UserInterface|Viewport|AddtoViewport _returnvalue_2 0)))

(fn ReturnfromAuction
  (bind _returnvalue (Game|Player|GetPlayerPawn 0))
  (bind _returnvalue_2 (Game|GetPlayerController 0))
  (bind _foundwidgets (Widget|GetAllWidgetsOfClass "/Game/Dynamic/Blueprints/WBP_DungeonView.WBP_DungeonView_C" true))
  (Variables|/Game/Dynamic/Blueprints/WBP_DungeonView.WBP_DungeonView_C|SetAuctionsCompleted (Utilities|Array|Get(acopy) _foundwidgets) (+ (Variables|/Game/Dynamic/Blueprints/WBP_DungeonView.WBP_DungeonView_C|GetAuctionsCompleted (Utilities|Array|Get(acopy) _foundwidgets)) 1))
  (Utilities|Casting|CastToBP_DungeonPawn _returnvalue)
  (if (Utilities|IsValid (Actor|GetComponentbyClass _returnvalue "/Script/Engine.CameraComponent"))
    (Game|Player|SetViewTargetwithBlend _returnvalue_2 (Pawn|GetControlledPawn _returnvalue_2) 0.0 "VTBlend_Linear" 0.0 false)
    (Input|SetInputModeGameandUI _returnvalue_2 0 "DoNotLock" true false)
    (bind _outactors (Actor|GetAllActorsOfClass "/Game/Dynamic/Blueprints/BP_UnitManager.BP_UnitManager_C"))
    (Default|ReActivateAuctions (Utilities|Array|Get(acopy) _outactors))))